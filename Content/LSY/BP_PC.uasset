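; BP_PC is a player controller that links a test UI widget to the game mode for sending a selected index over the network.
; On BeginPlay, non-server instances create UMG_Test, add it to the viewport and show the mouse cursor.
; ROS_SendIndexToServer passes the selected number to BP_GameMode, while ROC_WriteIndexToUI writes a received index into the widget's text.
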(event Custom|ROS_SendIndexToServer
  (params (SelectNumber :type Integer))
  (bind _asbp_game_mode (Utilities|Casting|CastToBP_GameMode (Game|GetGameMode)))
  (Default|ReceiveSelectIndex _asbp_game_mode SelectNumber))

(event Custom|ROC_WriteIndexToUI
  (params (RecieveIndex :type Integer))
  (Rendering|Components|TextRender|SetText (Variables|/Game/LSY/UMG_Test.UMG_Test_C|GetIndexText (Variables|Default|GetUI_Index)) (Utilities|Text|ToText(Integer) RecieveIndex)))

(event EventBeginPlay
  (Development|PrintString "Hello")
  (if (not (Networking|IsServer))
    (bind _returnvalue (UserInterface|CreateWidget "/Game/LSY/UMG_Test.UMG_Test_C"))
    (bind _output_get (Variables|Default|SetUI_Index _returnvalue))
    (UserInterface|Viewport|AddtoViewport _output_get 0)
    (Variables|Default|SetbShowMouseCursor true)))

(fn ConstructionScript)